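; Game mode Blueprint that sets up the turn-based HUD and shows the game-over screen.
; On BeginPlay it creates the end-turn and player-turn widgets and adds them to the viewport.
; The OnGameOver event creates a game-over widget, fills its text with the winning player's number and displays it.
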(event `self.ReceiveBeginPlay`
  (bind _returnvalue (`|CreateWidget` "/Game/Widgets/WBP_EndTurn.WBP_EndTurn_C"))
  (`UserWidget.AddToViewport` _returnvalue 0)
  (bind _returnvalue_2 (`|CreateWidget` "/Game/Widgets/WBP_PlayerTurn.WBP_PlayerTurn_C"))
  (`UserWidget.AddToViewport` _returnvalue_2 0))

(event `self.OnGameOver`
  (params (WinningPlayer :type Integer))
  (bind _returnvalue (`|CreateWidget` "/Game/Widgets/WBP_GameOver.WBP_GameOver_C"))
  (`TextBlock.SetText` (`/Game/Widgets/WBP_GameOver.GameOverText` _returnvalue) (`|FormatText` "Player {x} won!" (`KismetTextLibrary.Conv_IntToText` WinningPlayer)))
  (`UserWidget.AddToViewport` _returnvalue 0))

(fn `UserConstructionScript`)