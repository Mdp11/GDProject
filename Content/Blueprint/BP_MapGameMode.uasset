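; Game mode for map levels that manages per-level persistent map data and restores points of interest (PoI) at startup.
; On BeginPlay it loads the MapSavedData save object from the slot named after the current level, or creates a new one, then calls LoadPoI on it.
; SaveMapLevelData writes that object back to the same slot but is not called within this graph.
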(event `self.ReceiveBeginPlay`
  (`self.InitLevelSavedData`)
  (`/Game/Blueprint/MapSavedData.LoadPoI` (`self.MapSavedData`)))

(fn `InitLevelSavedData`
  (bind _returnvalue (`GameplayStatics.GetCurrentLevelName` true))
  (bind _returnvalue_2 (`GameplayStatics.DoesSaveGameExist` _returnvalue))
  (if _returnvalue_2
    (bind _returnvalue_3 (`GameplayStatics.GetCurrentLevelName` true))
    (bind _returnvalue_4 (`GameplayStatics.LoadGameFromSlot` _returnvalue_3))
    (bind _asmap_saved_data (cast `/Game/Blueprint/MapSavedData` _returnvalue_4))
    (set `self.MapSavedData` _asmap_saved_data)
    (else
      (bind _returnvalue_5 (`GameplayStatics.CreateSaveGameObject` "/Game/Blueprint/MapSavedData.MapSavedData_C"))
      (set `self.MapSavedData` _returnvalue_5))))

(fn `SaveMapLevelData`
  (bind _returnvalue (`GameplayStatics.GetCurrentLevelName` true))
  (`GameplayStatics.SaveGameToSlot` (`self.MapSavedData`) _returnvalue))

(fn `UserConstructionScript`)