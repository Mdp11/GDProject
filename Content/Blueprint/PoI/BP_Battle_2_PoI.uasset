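; Battle point-of-interest actor that decorates itself with scattered small stones and opens DefaultMap when clicked.
; On BeginPlay, AddMesh spawns static mesh components within a square around the Scene component, without shadows or collision.
; It guarantees the minimum count, then coin-flips each further element up to the maximum.
; Mesh choice, position, yaw and per-axis scale come from random streams seeded by the clock's milliseconds times a random float.
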(event `self.ReceiveBeginPlay`
  (`parent.ReceiveBeginPlay`)
  (`|ExecutionSequence`
    (:`then_0`
      (`self.AddMesh` (`|MakeArray` "/Game/Stylized_Forest/Meshes/stones/SM_small_stone_01.SM_small_stone_01" "/Game/Stylized_Forest/Meshes/stones/SM_small_stone_02.SM_small_stone_02" "/Game/Stylized_Forest/Meshes/stones/SM_small_stone_03.SM_small_stone_03" "/Game/Stylized_Forest/Meshes/stones/SM_small_stone_04.SM_small_stone_04" :!type "StaticMesh Object Reference") 10 5 5.0 8.0))))

(event `self.ReceiveActorOnClicked`
  (params (ButtonPressed :type "Key Structure"))
  (`GameplayStatics.OpenLevel` "DefaultMap"))

(fn `AddMesh`
  (params (Mesh :type "Array of StaticMesh Object Reference") (MaxElements :type Integer :default 1) (MinElements :type Integer) (MinScale :type "Float (double-precision)" :default 0.05) (MaxScale :type "Float (double-precision)" :default 0.2))
  (locals (PlacedElements :type Integer))
  (bind _returnvalue (`KismetMathLibrary.RandomFloatInRangeFromStream` MinScale MaxScale (`KismetMathLibrary.MakeRandomStream` (`KismetMathLibrary.FTrunc` (* (`KismetMathLibrary.GetMillisecond` (`KismetMathLibrary.Now`)) (`KismetMathLibrary.RandomFloat`))))))
  (for _ (range MaxElements)
    (if (< (`local.PlacedElements`) MinElements)
      (bind _returnvalue_2 (`AddComponent|NODE_AddStaticMeshComponent-2` :`RelativeTransform` (`KismetMathLibrary.MakeTransform` (`KismetMathLibrary.MakeVector` (`KismetMathLibrary.RandomFloatInRangeFromStream` -430.0 430.0 (`KismetMathLibrary.MakeRandomStream` (`KismetMathLibrary.FTrunc` (* (`KismetMathLibrary.GetMillisecond` (`KismetMathLibrary.Now`)) (`KismetMathLibrary.RandomFloat`))))) (`KismetMathLibrary.RandomFloatInRangeFromStream` -430.0 430.0 (`KismetMathLibrary.MakeRandomStream` (`KismetMathLibrary.FTrunc` (* (`KismetMathLibrary.GetMillisecond` (`KismetMathLibrary.Now`)) (`KismetMathLibrary.RandomFloat`)))))) (`KismetMathLibrary.MakeRotator` 0.0 0.0 (`KismetMathLibrary.RandomFloatInRangeFromStream` -180.0 180.0 (`KismetMathLibrary.MakeRandomStream` (`KismetMathLibrary.FTrunc` (* (`KismetMathLibrary.GetMillisecond` (`KismetMathLibrary.Now`)) (`KismetMathLibrary.RandomFloat`)))))) (`KismetMathLibrary.MakeVector` _returnvalue _returnvalue _returnvalue)) :!label _label))
      (`|ExecutionSequence`
        (:`then_0`
          (`StaticMeshComponent.SetStaticMesh` _returnvalue_2 (`|GetArrayItem` Mesh (`KismetMathLibrary.RandomIntegerInRangeFromStream` 0 (- (`KismetArrayLibrary.Array_Length` Mesh) 1) (`KismetMathLibrary.MakeRandomStream` (`KismetMathLibrary.FTrunc` (* (`KismetMathLibrary.GetMillisecond` (`KismetMathLibrary.Now`)) (`KismetMathLibrary.RandomFloat`))))))))
        (:`then_1`
          (`PrimitiveComponent.SetCastShadow` _returnvalue_2 false))
        (:`then_2`
          (`SceneComponent.K2_AttachToComponent` _returnvalue_2 (`self.Scene`) "None" "KeepRelative" "KeepRelative" "KeepRelative" true))
        (:`then_3`
          (`PrimitiveComponent.SetCollisionEnabled` _returnvalue_2 "NoCollision"))
        (:`then_4`
          (`/Engine/EditorBlueprintResources/StandardMacros.IncrementInt` (`local.PlacedElements`))))
      (elif (`KismetMathLibrary.RandomBool`)
        (goto _label)))))

(fn `UserConstructionScript`
  (`parent.UserConstructionScript`))